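; A functional test that checks whether a referenced Character can walk into a Trigger actor.
; After a one-second delay at start it applies a single downward movement input.
; Every tick it feeds forward input along the Character's facing plus a slight upward input.
; The test finishes as succeeded when the Character overlaps the Trigger, and the graph has no explicit failure path.
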(event `self.ReceiveStartTest`
  (`KismetSystemLibrary.Delay` 1.0)
  (`Pawn.AddMovementInput` (`self.Character`) (0.0 0.0 -50.0) 0.01 false))

(event `self.ReceiveTick`
  (params (DeltaSeconds :type "Float (single-precision)"))
  (bind _character (`self.Character`))
  (`Pawn.AddMovementInput` _character (`self.GetActorForwardVector` _character) 1.0 false)
  (`Pawn.AddMovementInput` (`self.Character`) (0.0 0.0 10.0) 0.01 false))

(event `self.Trigger.OnActorBeginOverlap`
  (params (OverlappedActor :type "Actor Object Reference") (OtherActor :type "Actor Object Reference"))
  (if (== OtherActor (`self.Character`))
    (`self.FinishTest` "Succeeded")))

(fn `UserConstructionScript`)