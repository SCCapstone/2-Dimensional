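; SpaceMan is the player's 2D flipbook character: it moves on two axes, fires projectiles in four directions and opens the pause menu.
; Fire inputs spawn BP_Projectile at per-direction arrow components with a blaster sound.
; Tick drains health while the capsule overlaps anything, otherwise updates the flipbook from movement and increments Score.
; Negative health sets IsDead, which disables input and shows the game-over HUD after a delay.
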(event `self.ReceiveBeginPlay`
  (set `self.IsDead` false)
  (set `self.Health` 100.0)
  (set `self.Score` 0.0))

(event `InputAction|Fire Down`
  (params (Key :type "Key Structure"))
  (:`Pressed`
    (`GameplayStatics.PlaySoundAtLocation` "/Game/Sounds/blaster_Cue.blaster_Cue" (`self.K2_GetActorLocation`) (struct) 1.0 1.0 0.0 null null null)))

(event `InputAction|Fire Down`
  (params (Key :type "Key Structure"))
  (:`Pressed`
    (`|SpawnActorFromClass` "/Game/Blueprints/BP_Projectile.BP_Projectile_C" (`SceneComponent.K2_GetComponentToWorld` (`self.Arrow Down`)) "Undefined" "OverrideRootScale" self null)))

(event `InputAction|Fire Up`
  (params (Key :type "Key Structure"))
  (:`Pressed`
    (`GameplayStatics.PlaySoundAtLocation` "/Game/Sounds/blaster_Cue.blaster_Cue" (`self.K2_GetActorLocation`) (struct) 1.0 1.0 0.0 null null null)))

(event `InputAction|Fire Up`
  (params (Key :type "Key Structure"))
  (:`Pressed`
    (`|SpawnActorFromClass` "/Game/Blueprints/BP_Projectile.BP_Projectile_C" (`SceneComponent.K2_GetComponentToWorld` (`self.Arrow Up`)) "Undefined" "OverrideRootScale" self null)))

(event `InputAction|Fire Left`
  (params (Key :type "Key Structure"))
  (:`Pressed`
    (`GameplayStatics.PlaySoundAtLocation` "/Game/Sounds/blaster_Cue.blaster_Cue" (`self.K2_GetActorLocation`) (struct) 1.0 1.0 0.0 null null null)))

(event `InputAction|Fire Left`
  (params (Key :type "Key Structure"))
  (:`Pressed`
    (`|SpawnActorFromClass` "/Game/Blueprints/BP_Projectile.BP_Projectile_C" (`SceneComponent.K2_GetComponentToWorld` (`self.Arrow Left`)) "Undefined" "OverrideRootScale" self null)))

(event `InputAction|Fire Right`
  (params (Key :type "Key Structure"))
  (:`Pressed`
    (`GameplayStatics.PlaySoundAtLocation` "/Game/Sounds/blaster_Cue.blaster_Cue" (`self.K2_GetActorLocation`) (struct) 1.0 1.0 0.0 null null null)))

(event `InputAction|Fire Right`
  (params (Key :type "Key Structure"))
  (:`Pressed`
    (`|SpawnActorFromClass` "/Game/Blueprints/BP_Projectile.BP_Projectile_C" (`SceneComponent.K2_GetComponentToWorld` (`self.Arrow Right`)) "Undefined" "OverrideRootScale" self null)))

(event `InputAxis|UpDown`
  (params (AxisValue :type "Float (single-precision)"))
  (`self.AddMovementInput` (0.0 -1.0 0.0) AxisValue))

(event `Key|P`
  (params (Key :type "Key Structure"))
  (:`Pressed`
    (bind _returnvalue (`|CreateWidget` "/Game/Blueprints/PauseMenu/PauseMenuWidget.PauseMenuWidget_C"))
    (`UserWidget.AddToViewport` _returnvalue 0)
    (`GameplayStatics.SetGamePaused` true)))

(event `InputAxis|LeftRight`
  (params (AxisValue :type "Float (single-precision)"))
  (`self.AddMovementInput` (1.0 0.0 0.0) AxisValue))

(event `self.ReceiveTick`
  (params (DeltaSeconds :type "Float (single-precision)"))
  (if (`self.IsDead`)
    (`/Engine/EditorBlueprintResources/StandardMacros.DoOnce` false
      (:`Completed`
        (`self.DisableInput` null)
        (`KismetSystemLibrary.Delay` 1.0)
        (bind _returnvalue (`|CreateWidget` "/Game/Blueprints/HUD_GameOver.HUD_GameOver_C"))
        (`UserWidget.AddToViewport` _returnvalue 0)))
    (elif (< (`self.Health`) 0.0)
      (set `self.IsDead` true)
      (`GameplayStatics.PlaySoundAtLocation` "/Game/Sounds/game_over_Cue.game_over_Cue" (`self.K2_GetActorLocation`) (struct) 1.0 1.0 0.0 null null null)
      (elif (`self.IsOverlapping`)
        (bind _output_get (set `self.Health` (- (stale _output_get) 1.0)))
        (`GameplayStatics.PlaySoundAtLocation` "/Game/Sounds/taking_damage_Cue.taking_damage_Cue" (`self.K2_GetActorLocation`) (struct) 1.0 1.0 0.0 null null null)
        (else
          (`self.SetFlipBook`)
          (bind _output_get_2 (set `self.Score` (+ (stale _output_get_2) 1.0))))))))

(event `self.CapsuleComponent.OnComponentBeginOverlap`
  (params (OverlappedComponent :type "PrimitiveComponent Object Reference") (OtherActor :type "Actor Object Reference") (OtherComp :type "PrimitiveComponent Object Reference") (OtherBodyIndex :type Integer) (bFromSweep :type Boolean) (SweepResult :type "HitResult Structure (by ref)"))
  (set `self.IsOverlapping` true))

(event `self.CapsuleComponent.OnComponentEndOverlap`
  (params (OverlappedComponent :type "PrimitiveComponent Object Reference") (OtherActor :type "Actor Object Reference") (OtherComp :type "PrimitiveComponent Object Reference") (OtherBodyIndex :type Integer))
  (set `self.IsOverlapping` false))

(fn `SetFlipBook`
  (bind _lastdir (`self.LastDir`))
  (if (or (!= (`self.GetInputAxisValue`) 0.0) (!= (`self.GetInputAxisValue`) 0.0))
    (set `self.LastDir` (select `bool` (> (`self.GetInputAxisValue`) 0.0) :`false` (select `bool` (< (`self.GetInputAxisValue`) 0.0) :`false` (select `bool` (> (`self.GetInputAxisValue`) 0.0) :`false` "NewEnumerator2" :`true` "NewEnumerator3" :!type "/Game/Spaceman/MoveDirection Enum") :`true` "NewEnumerator1") :`true` "NewEnumerator0"))
    (`PaperFlipbookComponent.SetFlipbook` (`self.Sprite`) (select `bool` (> (`KismetMathLibrary.VSize` (`self.GetVelocity`)) 0.0) :`false` (select `/Game/Spaceman/MoveDirection` _lastdir :`NewEnumerator0` "/Game/Spaceman/Idle.Idle" :`NewEnumerator1` "/Game/Spaceman/Idle.Idle" :`NewEnumerator2` "/Game/Spaceman/IdleLeft.IdleLeft" :`NewEnumerator3` "/Game/Spaceman/Idle.Idle" :!type "PaperFlipbook Object Reference") :`true` (select `/Game/Spaceman/MoveDirection` _lastdir :`NewEnumerator0` "/Game/Spaceman/Idle.Idle" :`NewEnumerator1` "/Game/Spaceman/Idle.Idle" :`NewEnumerator2` "/Game/Spaceman/WalkLeftFB.WalkLeftFB" :`NewEnumerator3` "/Game/Spaceman/WalkRight.WalkRight" :!type "PaperFlipbook Object Reference")))))

(fn `UserConstructionScript`)