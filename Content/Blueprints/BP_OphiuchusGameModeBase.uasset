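; BP_OphiuchusGameModeBase is a game mode that runs a minute-and-second countdown and ends the game when it expires.
; Tick feeds a one-second Delay, so Sec drops about once per second and rolls over into Min.
; At zero, a DoOnce disables input, pauses the game, adds the HUD_GameOver widget and shows the mouse cursor.
; An L key binding raises Min to a high value, apparently as a debug shortcut.
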(event `self.ReceiveTick`
  (params (DeltaSeconds :type "Float (single-precision)"))
  (`KismetSystemLibrary.Delay` 1.0)
  (if (== (`self.sec`) 0)
    (if (== (`self.min`) 0)
      (`/Engine/EditorBlueprintResources/StandardMacros.DoOnce` false
        (:`Completed`
          (`self.DisableInput` null)
          (`GameplayStatics.SetGamePaused` true)
          (bind _returnvalue (`|CreateWidget` "/Game/Blueprints/HUD_GameOver.HUD_GameOver_C"))
          (`UserWidget.AddToViewport` _returnvalue 0)
          (set `PlayerController.bShowMouseCursor` true (`GameplayStatics.GetPlayerController` 0))))
      (else
        (set `self.sec` 59)
        (set `self.min` (- (`self.min`) 1))))
    (else
      (set `self.sec` (- (`self.sec`) 1)))))

(event `Key|L`
  (params (Key :type "Key Structure"))
  (:`Pressed`
    (set `self.min` 99)))

(fn `UserConstructionScript`)