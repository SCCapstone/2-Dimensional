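; BasicEnemy_BP is a basic enemy that damages the SpaceMan player on contact.
; When its capsule begins overlapping a SpaceMan and it is not dead, it waits briefly, then subtracts a fixed amount from the player character's Health.
; Damage applies once per overlap and does not recheck contact after the delay.
; IsOverlapping tracks contact but is not read here, and IsDead is only reset on BeginPlay.
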(event `self.ReceiveBeginPlay`
  (set `self.IsDead` false))

(event `self.Capsule.OnComponentBeginOverlap`
  (params (OverlappedComponent :type "PrimitiveComponent Object Reference") (OtherActor :type "Actor Object Reference") (OtherComp :type "PrimitiveComponent Object Reference") (OtherBodyIndex :type Integer) (bFromSweep :type Boolean) (SweepResult :type "HitResult Structure (by ref)"))
  (cast `/Game/Spaceman/SpaceMan` OtherActor)
  (set `self.IsOverlapping` true)
  (if (not (`self.IsDead`))
    (bind _asspace_man (cast `/Game/Spaceman/SpaceMan` (`GameplayStatics.GetPlayerCharacter` 0)))
    (`KismetSystemLibrary.Delay` 0.1)
    (set `/Game/Spaceman/SpaceMan.Health` (- (`/Game/Spaceman/SpaceMan.Health` _asspace_man) 10.0) _asspace_man)))

(event `self.Capsule.OnComponentEndOverlap`
  (params (OverlappedComponent :type "PrimitiveComponent Object Reference") (OtherActor :type "Actor Object Reference") (OtherComp :type "PrimitiveComponent Object Reference") (OtherBodyIndex :type Integer))
  (cast `/Game/Spaceman/SpaceMan` OtherActor)
  (set `self.IsOverlapping` false))

(fn `UserConstructionScript`)