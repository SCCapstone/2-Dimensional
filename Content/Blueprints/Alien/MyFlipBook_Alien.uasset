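; Alien actor Blueprint with a capsule component, set up as the start of a contact-damage enemy against SpaceMan.
; BeginPlay clears the IsOverlapping flag, while Tick and the capsule overlap events have no logic connected.
; Disconnected nodes would set that flag on SpaceMan overlap and subtract from its Health with a Delay, but none of them run, so the alien deals no damage here.
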(event `self.ReceiveBeginPlay`
  (set `self.IsOverlapping` false))

(event `self.ReceiveTick`
  (params (DeltaSeconds :type "Float (single-precision)")))

(event `self.CapsuleComponent.OnComponentBeginOverlap`
  (params (OverlappedComponent :type "PrimitiveComponent Object Reference") (OtherActor :type "Actor Object Reference") (OtherComp :type "PrimitiveComponent Object Reference") (OtherBodyIndex :type Integer) (bFromSweep :type Boolean) (SweepResult :type "HitResult Structure (by ref)")))

(event `self.CapsuleComponent.OnComponentEndOverlap`
  (params (OverlappedComponent :type "PrimitiveComponent Object Reference") (OtherActor :type "Actor Object Reference") (OtherComp :type "PrimitiveComponent Object Reference") (OtherBodyIndex :type Integer)))

(fn `UserConstructionScript`)