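; BasicEnemy_BP is a basic alien enemy, with egg death audio, that takes damage and rewards the player when killed.
; AnyDamage subtracts from Health and calls Death at zero, which destroys the actor and plays the sound at its location.
; Death then casts the player to SpaceMan and, only if Ammo is at most 100, grants ammo, score scaled by prior EggKills, and a kill increment.
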(event `self.ReceiveAnyDamage`
  (params (Damage :type "Float (single-precision)") (DamageType :type "DamageType Object Reference") (InstigatedBy :type "Controller Object Reference") (DamageCauser :type "Actor Object Reference"))
  (set `self.Health` (- (`self.Health`) Damage))
  (if (<= (`self.Health`) 0.0)
    (`self.Death`)))

(event `Death`
  (`self.K2_DestroyActor`)
  (`GameplayStatics.PlaySoundAtLocation` "/Game/Sounds/egg_death_Cue.egg_death_Cue" (`self.K2_GetActorLocation`) (struct) 1.0 1.0 0.0 null null null)
  (bind _asspace_man (cast `/Game/Blueprints/Spaceman/SpaceMan` (`GameplayStatics.GetPlayerCharacter` 0)))
  (if (<= (`/Game/Blueprints/Spaceman/SpaceMan.Ammo` _asspace_man) 100.0)
    (set `/Game/Blueprints/Spaceman/SpaceMan.Ammo` (+ (`/Game/Blueprints/Spaceman/SpaceMan.Ammo` _asspace_man) 20.0) _asspace_man)
    (bind _output_get (set `/Game/Blueprints/Spaceman/SpaceMan.Score` (+ (stale _output_get) (* (`KismetMathLibrary.FTrunc` (`/Game/Blueprints/Spaceman/SpaceMan.EggKills` _asspace_man)) 100.0)) _asspace_man))
    (bind _output_get_2 (set `/Game/Blueprints/Spaceman/SpaceMan.EggKills` (+ (stale _output_get_2) 1.0) _asspace_man))))

(fn `UserConstructionScript`)